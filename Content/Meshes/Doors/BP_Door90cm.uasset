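; VR-style 90 cm door that opens by grabbing its handle with the left or right hand, with events to swap between panel meshes A–H.
; While held, a grasping hand mesh shows and pivot yaw follows the hand position, clamped to 90 degrees; left updates on Tick, right on each hold event call.
; Releasing past 15 degrees plays a timeline that swings it open and locks further movement.
; BeginPlay poses the left hand and corrects hand scale on mirrored doors.
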(event `self.ReceiveBeginPlay`
  (bind _returnvalue_x (`KismetMathLibrary.BreakVector` (`SceneComponent.K2_GetComponentScale` (`self.DefaultSceneRoot`))))
  (bind _asabp_hand_anim (cast `/Game/Character/ABP_HandAnim` (`SkeletalMeshComponent.GetAnimInstance` (`self.HandLeft`))))
  (set `/Game/Character/ABP_HandAnim.GraspValue` 1.0 _asabp_hand_anim)
  ;[1 1 1] Fix Hands Scale
  (if (< _returnvalue_x 0.0)
    (`SceneComponent.SetRelativeScale3D` (`self.HandRight`) (-1.0 1.0 1.0))
    (`SceneComponent.SetRelativeScale3D` (`self.HandLeft`) (-1.0 1.0 1.0))))

(event `self.ReceiveTick`
  (params (DeltaSeconds :type "Float (single-precision)"))
  (bind _doorhandlecomponent (`self.DoorHandleComponent`))
  (`|ExecutionSequence`
    (:`then_1`
      ;[0.3968 0.9647 1] Left Hand
      ;;[1 1 1] Hold and Open Door
      (if (stale `/Game/Character/BPI_DoorOpening.HoldingHandleByLeft` _output_get)
        (`SceneComponent.SetVisibility` (`self.HandLeft`) true false)
        (if (not (`self.IsDoorOpen`))
          (bind (_returnvalue_roll _returnvalue_pitch _returnvalue_yaw) (`KismetMathLibrary.BreakRotator` (`KismetMathLibrary.FindLookAtRotation` (- (`KismetMathLibrary.Vector_GetAbs` (`SceneComponent.K2_GetComponentLocation` _doorhandlecomponent)) (`KismetMathLibrary.Vector_GetAbs` (`SceneComponent.K2_GetComponentLocation` (stale `/Game/Character/BPI_DoorOpening.HoldingHandleByLeft` Hand)))) (`SceneComponent.RelativeLocation` _doorhandlecomponent))))
          (`SceneComponent.K2_SetRelativeRotation` (`self.Pivot`) (`KismetMathLibrary.MakeRotator` 0.0 0.0 (`KismetMathLibrary.ClampAngle` (`KismetMathLibrary.Abs` (+ _returnvalue_yaw 30.0)) 0.0 90.0)) false false))))))

(event `/Game/Character/BPI_DoorOpening.HoldingHandleByRight`
  (params (Hand :type "SceneComponent Object Reference"))
  (bind _doorhandlecomponent (`self.DoorHandleComponent`))
  (bind (_returnvalue_roll _returnvalue_pitch _returnvalue_yaw) (`KismetMathLibrary.BreakRotator` (`KismetMathLibrary.FindLookAtRotation` (- (`KismetMathLibrary.Vector_GetAbs` (`SceneComponent.K2_GetComponentLocation` _doorhandlecomponent)) (`KismetMathLibrary.Vector_GetAbs` (`SceneComponent.K2_GetComponentLocation` Hand))) (`SceneComponent.RelativeLocation` _doorhandlecomponent))))
  ;[0.3968 0.9647 1] Right Hand
  ;;[1 1 1] Hold and Open Door
  (bind _output_get (set `self.DoorHanldeIsHeldByRight` true))
  (if _output_get
    (`SceneComponent.SetVisibility` (`self.HandRight`) true false)
    (if (not (`self.IsDoorOpen`))
      (`SceneComponent.K2_SetRelativeRotation` (`self.Pivot`) (`KismetMathLibrary.MakeRotator` 0.0 0.0 (`KismetMathLibrary.ClampAngle` (`KismetMathLibrary.Abs` (+ _returnvalue_yaw 30.0)) 0.0 90.0)) false false))))

(event `/Game/Character/BPI_DoorOpening.HoldingHandleByLeft`
  (params (Hand :type "SceneComponent Object Reference"))
  ;[0.3968 0.9647 1] Left Hand
  ;;[1 1 1] Hold and Open Door
  (bind _output_get (set `self.DoorHanldeIsHeldByLeft` true)))

(event `/Game/Character/BPI_DoorOpening.DropHandleByRight`
  (params (Hand :type "SceneComponent Object Reference"))
  (bind (_relativerotation_roll _relativerotation_pitch _relativerotation_yaw) (`KismetMathLibrary.BreakRotator` (`SceneComponent.RelativeRotation` (`self.Pivot`))))
  ;[0.3968 0.9647 1] Right Hand
  ;;[1 1 1] Release Door
  (`SceneComponent.SetVisibility` (`self.HandRight`) false false)
  (set `self.DoorHanldeIsHeldByRight` false)
  (if (> _relativerotation_yaw 15.0)
    (if (not (`self.IsDoorOpen`))
      (`Timeline|DoorAmimOpening`
        (:`Update`
          (if (not (`KismetMathLibrary.NearlyEqual_FloatFloat` _relativerotation_yaw 90.0 2.0))
            (`SceneComponent.K2_AddRelativeRotation` (`self.Pivot`) (`KismetMathLibrary.MakeRotator` 0.0 0.0 3.0) false false)))
        (:`Finished`
          (set `self.IsDoorOpen` true))))))

(event `/Game/Character/BPI_DoorOpening.DropHandleByLeft`
  (params (Hand :type "SceneComponent Object Reference"))
  (bind (_relativerotation_roll _relativerotation_pitch _relativerotation_yaw) (`KismetMathLibrary.BreakRotator` (`SceneComponent.RelativeRotation` (`self.Pivot`))))
  ;[0.3968 0.9647 1] Left Hand
  ;;[1 1 1] Release Door
  (`SceneComponent.SetVisibility` (`self.HandLeft`) false false)
  (set `self.DoorHanldeIsHeldByLeft` false)
  (if (> _relativerotation_yaw 15.0)
    (if (not (`self.IsDoorOpen`))
      (`Timeline|Timeline`
        (:`Update`
          (if (not (`KismetMathLibrary.NearlyEqual_FloatFloat` _relativerotation_yaw 90.0 2.0))
            (`SceneComponent.K2_AddRelativeRotation` (`self.Pivot`) (`KismetMathLibrary.MakeRotator` 0.0 0.0 3.0) false false)))
        (:`Finished`
          (set `self.IsDoorOpen` true))))))

(event `/Game/Character/Widgets/BPI_ModifyDoorPanel.DoorType-A`
  (`StaticMeshComponent.SetStaticMesh` (`self.Panel`) "/Game/Meshes/Doors/SM_Door_90cm_Panel.SM_Door_90cm_Panel"))

(event `/Game/Character/Widgets/BPI_ModifyDoorPanel.DoorType-B`
  (`StaticMeshComponent.SetStaticMesh` (`self.Panel`) "/Game/Meshes/Doors/SM_DoorPanelTypeB.SM_DoorPanelTypeB"))

(event `/Game/Character/Widgets/BPI_ModifyDoorPanel.DoorType-C`
  (`StaticMeshComponent.SetStaticMesh` (`self.Panel`) "/Game/Meshes/Doors/SM_DoorPanelTypeC.SM_DoorPanelTypeC"))

(event `/Game/Character/Widgets/BPI_ModifyDoorPanel.DoorType-D`
  (`StaticMeshComponent.SetStaticMesh` (`self.Panel`) "/Game/Meshes/Doors/SM_DoorPanelTypeD.SM_DoorPanelTypeD"))

(event `/Game/Character/Widgets/BPI_ModifyDoorPanel.DoorType-E`
  (`StaticMeshComponent.SetStaticMesh` (`self.Panel`) "/Game/Meshes/Doors/SM_DoorPanelTypeE.SM_DoorPanelTypeE"))

(event `/Game/Character/Widgets/BPI_ModifyDoorPanel.DoorType-F`
  (`StaticMeshComponent.SetStaticMesh` (`self.Panel`) "/Game/Meshes/Doors/SM_DoorPanelTypeF.SM_DoorPanelTypeF"))

(event `/Game/Character/Widgets/BPI_ModifyDoorPanel.DoorType-G`
  (`StaticMeshComponent.SetStaticMesh` (`self.Panel`) "/Game/Meshes/Doors/SM_DoorPanelTypeG.SM_DoorPanelTypeG"))

(event `/Game/Character/Widgets/BPI_ModifyDoorPanel.DoorType-H`
  (`StaticMeshComponent.SetStaticMesh` (`self.Panel`) "/Game/Meshes/Doors/SM_DoorPanelTypeH.SM_DoorPanelTypeH"))

(fn `UserConstructionScript`)