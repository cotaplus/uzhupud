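; Office glass wall actor with a sliding door dragged by a right hand, plus a scale animation that removes the wall.
; While held, a proxy hand shows and the frame follows clamped hand travel from the grab point, sign-corrected by actor facing; the axis branch is hardwired to world Y.
; Release hides the hand and a timeline nudges the door open, then locks it.
; ScaleWall animates the pivot's Y scale, then destroys the wall meshes.
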(event `self.ReceiveTick`
  (params (DeltaSeconds :type "Float (single-precision)")))

(event `/Game/Character/BPI_DoorOpening.HoldingHandleByRight`
  (params (Hand :type "SceneComponent Object Reference"))
  (bind (_returnvalue_roll _returnvalue_pitch _returnvalue_yaw) (`KismetMathLibrary.BreakRotator` (`SceneComponent.K2_GetComponentRotation` Hand)))
  (bind _returnvalue (`SceneComponent.K2_GetComponentLocation` Hand))
  (bind _righthand (`self.RightHand`))
  (bind (_returnvalue_x _returnvalue_y) (`KismetMathLibrary.BreakVector` (`SceneComponent.GetForwardVector` (`self.DefaultSceneRoot`))))
  (bind (_returnvalue_x_2 _returnvalue_y_2) (`KismetMathLibrary.BreakVector` (`SceneComponent.K2_GetComponentLocation` _righthand)))
  (bind _returnvalue_x_3 (`KismetMathLibrary.BreakVector` (- (`self.HandLocationStart`) (`self.HandLocationUpdated`))))
  (bind (_returnvalue_x_4 _returnvalue_y_3) (`KismetMathLibrary.BreakVector` (- (`self.HandLocationStart`) (`self.HandLocationUpdated`))))
  (`|ExecutionSequence`
    (:`then_0`
      (set `self.HandLocationUpdated` _returnvalue)
      (`SceneComponent.SetVisibility` _righthand true false)
      (if (not (`self.IsDoorOpen`))
        (`SceneComponent.K2_SetWorldRotation` (`self.HandPivot`) (`KismetMathLibrary.MakeRotator` 0.0 0.0 (/ _returnvalue_yaw 2.0)) false false)
        (if true
          (if (< _returnvalue_x 0.0)
            (set `self.SlideDirectionSwitch` 1.0)
            (else
              (set `self.SlideDirectionSwitch` -1.0)))
          (`SceneComponent.K2_SetRelativeLocation` (`self.SM_OfficeGlassWall_DoorFrame`) (`KismetMathLibrary.MakeVector` -5.138729 (- (`KismetMathLibrary.FClamp` (* _returnvalue_y_3 (`self.SlideDirectionSwitch`)) 0.0 85.0) 269.788074) -120.0) false false)
          (else
            (if (< 0.0 _returnvalue_y)
              (set `self.SlideDirectionSwitch` 1.0)
              (else
                (set `self.SlideDirectionSwitch` -1.0)))
            (`SceneComponent.K2_SetRelativeLocation` (`self.SM_OfficeGlassWall_DoorFrame`) (`KismetMathLibrary.MakeVector` 0.0 (`KismetMathLibrary.FClamp` (* _returnvalue_x_3 (`self.SlideDirectionSwitch`)) 0.0 85.0)) false false)))))
    (:`then_1`
      (`/Engine/EditorBlueprintResources/StandardMacros.DoOnce` false :!label _label
        (:`Completed`
          (set `self.HandLocationStart` _returnvalue)
          (if (not (`self.IsDoorOpen`))
            (`SceneComponent.K2_SetWorldLocation` _righthand (`KismetMathLibrary.MakeVector` _returnvalue_x_2 _returnvalue_y_2 (.z _returnvalue)) false false)))))))

(event `/Game/Character/BPI_DoorOpening.DropHandleByRight`
  (params (Hand :type "SceneComponent Object Reference"))
  (bind _sm_officeglasswall_doorframe (`self.SM_OfficeGlassWall_DoorFrame`))
  (bind (_relativelocation_x _relativelocation_y) (`KismetMathLibrary.BreakVector` (`SceneComponent.RelativeLocation` _sm_officeglasswall_doorframe)))
  (set `self.Temporal` false)
  (`|ExecutionSequence`
    (:`then_0`
      (`SceneComponent.SetVisibility` (`self.RightHand`) false false)
      (if (not (`self.IsDoorOpen`))
        (`Timeline|DoorSlideAssistance`
          (:`Update`
            (if (not (`KismetMathLibrary.NearlyEqual_FloatFloat` _relativelocation_y (- 85.0 269.788074) 2.0))
              (`SceneComponent.K2_AddRelativeLocation` _sm_officeglasswall_doorframe (0.0 2.0 0.0) false false)))
          (:`Finished`
            (set `self.IsDoorOpen` true)))))
    (:`then_1`
      (goto _label :!via `Reset`))))

(event `/Game/Meshes/Office/BPI_ScaleOfficeWalls.ScaleWall`
  (bind (_direction _scale) (`Timeline|Animation` :!via `PlayFromStart`)
    (:`Update`
      (`SceneComponent.SetRelativeScale3D` (`self.ScalePivot`) (`KismetMathLibrary.MakeVector` 1.0 _scale 1.0)))
    (:`Finished`
      (`ActorComponent.K2_DestroyComponent` (`self.SM_OfficeGlassWall_WallGlass`))
      (`ActorComponent.K2_DestroyComponent` (`self.SM_OfficeGlassWall_WallFrame`)))))

(fn `UserConstructionScript`)