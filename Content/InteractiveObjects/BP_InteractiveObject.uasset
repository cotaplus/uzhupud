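; Interactive physics object that can be picked up and dropped through separate left-hand and right-hand events, which share identical logic.
; On hold, it attaches to the given hand component, restores the mesh's pre-grab world location so it keeps its offset instead of snapping, then disables physics simulation.
; On drop, it detaches while keeping its world transform and re-enables physics on the mesh.
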(event `/Game/Character/BPI_Interactivity.HoldingObjectByLeft`
  (params (Hand :type "SceneComponent Object Reference") (HandLocation :type "Vector Structure"))
  (set `self.RealLocation` (+ (* (- HandLocation (`SceneComponent.K2_GetComponentLocation` (`self.Mesh`))) (`KismetMathLibrary.MakeVector` -1.0 -1.0 -1.0)) HandLocation))
  (`self.K2_AttachToComponent` Hand "None" "SnapToTarget" "KeepWorld" "KeepRelative")
  (`SceneComponent.K2_SetWorldLocation` (`self.Mesh`) (`self.RealLocation`) false false)
  (`PrimitiveComponent.SetSimulatePhysics` (`self.Mesh`) false))

(event `/Game/Character/BPI_Interactivity.DropObjectByLeft`
  (params (Hand :type "SceneComponent Object Reference"))
  (`self.K2_DetachFromActor` "KeepWorld" "KeepWorld")
  (`PrimitiveComponent.SetSimulatePhysics` (`self.Mesh`) true))

(event `/Game/Character/BPI_Interactivity.HoldingObjectByRight`
  (params (Hand :type "SceneComponent Object Reference") (HandLocation :type "Vector Structure"))
  (set `self.RealLocation` (+ (* (- HandLocation (`SceneComponent.K2_GetComponentLocation` (`self.Mesh`))) (`KismetMathLibrary.MakeVector` -1.0 -1.0 -1.0)) HandLocation))
  (`self.K2_AttachToComponent` Hand "None" "SnapToTarget" "KeepWorld" "KeepRelative")
  (`SceneComponent.K2_SetWorldLocation` (`self.Mesh`) (`self.RealLocation`) false false)
  (`PrimitiveComponent.SetSimulatePhysics` (`self.Mesh`) false))

(event `/Game/Character/BPI_Interactivity.DropObjectByRight`
  (params (Hand :type "SceneComponent Object Reference"))
  (`self.K2_DetachFromActor` "KeepWorld" "KeepWorld")
  (`PrimitiveComponent.SetSimulatePhysics` (`self.Mesh`) true))

(fn `UserConstructionScript`)